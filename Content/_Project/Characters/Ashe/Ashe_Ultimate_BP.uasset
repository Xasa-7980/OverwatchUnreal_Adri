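; Ashe's ultimate ability, which spawns a Bob_BP at the owning character's capsule with a vertical offset and matching yaw.
; Fire spawns only if not colliding; on success it stores the Bob reference, runs the parent fire, empties the charge and UI, and finishes after five seconds.
; A failed spawn only prints a message, keeping the charge.
; Update also finishes the ability in one state if Bob is no longer valid.
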(event `self.Fire`
  (bind _returnvalue (`SceneComponent.K2_GetComponentToWorld` (`Character.CapsuleComponent` (`self.OwningCharacter`))))
  (bind _returnvalue_2 (`|SpawnActorFromClass` "/Game/_Project/Characters/Ashe/Bob_BP.Bob_BP_C" (`KismetMathLibrary.MakeTransform` (+ (.location _returnvalue) (`KismetMathLibrary.MakeVector` 0.0 0.0 (`self.SpawnOffset`))) (`KismetMathLibrary.MakeRotator` 0.0 0.0 (.yaw (.rotation _returnvalue))) (.scale _returnvalue)) "DontSpawnIfColliding" "MultiplyWithRoot" null null))
  (`/Engine/EditorBlueprintResources/StandardMacros.IsValid` _returnvalue_2
    (:`Is Valid`
      (set `self.BobRef` _returnvalue_2)
      (`|ExecutionSequence`
        (:`then_0`
          (`parent.Fire`)
          (bind _output_get (set `self.CurrentCharge` 0.0))
          (`/Game/_Project/CommonSystems/Character_UI/BaseUI/Ultimate/Ultimate_UI.SetUltimateAmount` (`self.UltimateUI`) _output_get))
        (:`then_1`
          (`KismetSystemLibrary.Delay` 5.0)
          (`self.Finish`))))
    (:`Is Not Valid`
      (`KismetSystemLibrary.PrintString` "CAnt spawn bob"))))

(event `self.Update`
  (params (DeltaTime :type "Float (double-precision)"))
  (`parent.Update` 0.0)
  (if (`|EnumEquality` (`self.State`) "NewEnumerator2")
    (`/Engine/EditorBlueprintResources/StandardMacros.IsValid` (`self.BobRef`)
      (:`Is Not Valid`
        (`self.Finish`)))))