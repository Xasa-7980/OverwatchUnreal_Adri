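; Bob_BP is Bob, an AI-driven actor in the Ashe character folder that charges into things and tracks dummies within shooting range.
; On a roughly head-on hit while Bob_AIController is running, it launches any hit Character forward and sharply upward, then calls the controller's OnCollide for any obstacle.
; ShootRange overlap events maintain the DummiesInRange list, with no firing logic in this Blueprint.
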(event `self.ReceiveHit`
  (params (MyComp :type "PrimitiveComponent Object Reference") (Other :type "Actor Object Reference") (OtherComp :type "PrimitiveComponent Object Reference") (bSelfMoved :type Boolean) (HitLocation :type "Vector Structure") (HitNormal :type "Vector Structure") (NormalImpulse :type "Vector Structure") (Hit :type "HitResult Structure (by ref)"))
  (if (and (< (`KismetMathLibrary.Dot_VectorVector` HitNormal (`self.GetActorForwardVector`)) -0.5) (`/Game/_Project/Characters/Ashe/Bob_AIController.IsRunning?` (cast `/Game/_Project/Characters/Ashe/Bob_AIController` (`self.GetController`) :!pure true)))
    (`|ExecutionSequence`
      (:`then_0`
        (bind _ascharacter (cast `Character` Other))
        (`self.LaunchCharacter` _ascharacter (+ (* (`self.GetActorForwardVector`) 200.0) (0.0 0.0 1500.0)) false false))
      (:`then_1`
        (`/Game/_Project/Characters/Ashe/Bob_AIController.OnCollide` (cast `/Game/_Project/Characters/Ashe/Bob_AIController` (`self.GetController`) :!pure true))))))

(event `self.ShootRange.OnComponentBeginOverlap`
  (params (OverlappedComponent :type "PrimitiveComponent Object Reference") (OtherActor :type "Actor Object Reference") (OtherComp :type "PrimitiveComponent Object Reference") (OtherBodyIndex :type Integer) (bFromSweep :type Boolean) (SweepResult :type "HitResult Structure (by ref)"))
  (bind _asdummy (cast `/Game/_Project/Characters/Dummy/Dummy` OtherActor))
  (`BlueprintSetLibrary.Set_Add` (`self.DummiesInRange`) _asdummy))

(event `self.ShootRange.OnComponentEndOverlap`
  (params (OverlappedComponent :type "PrimitiveComponent Object Reference") (OtherActor :type "Actor Object Reference") (OtherComp :type "PrimitiveComponent Object Reference") (OtherBodyIndex :type Integer))
  (bind _asdummy (cast `/Game/_Project/Characters/Dummy/Dummy` OtherActor))
  (`BlueprintSetLibrary.Set_Remove` (`self.DummiesInRange`) _asdummy))

(fn `UserConstructionScript`)