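; Junkrat's weapon projectile, a bouncing shot that destroys itself on hitting a Dummy or on reaching its bounce limit.
; All logic runs from the ProjectileMovement bounce event, which casts the hit actor to Dummy and otherwise increments BounceCount against MaxBounces.
; Debug prints report bounces and Dummy hits, and the graph applies no damage or explosion.
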(event `self.ProjectileMovement.OnProjectileBounce`
  (params (ImpactResult :type "HitResult Structure (by ref)") (ImpactVelocity :type "Vector Structure (by ref)"))
  (`KismetSystemLibrary.PrintString` "boing")
  (cast `/Game/_Project/Characters/Dummy/Dummy` ImpactResult_HitActor
    (:`then`
      (`KismetSystemLibrary.PrintString` "It's a dummy")
      (`self.K2_DestroyActor` :!label _label))
    (:`CastFailed`
      (bind _result (`/Engine/EditorBlueprintResources/StandardMacros.IncrementInt` (`self.BounceCount`))
        (:`  `
          (if (>= _result (`self.MaxBounces`))
            (goto _label)))))))

(fn `UserConstructionScript`
  (`parent.UserConstructionScript`))