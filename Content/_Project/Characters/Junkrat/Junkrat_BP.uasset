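; Junkrat character Blueprint, a playable hero with a trap skill and an Expansive Force skill.
; On BeginPlay it sets its health, then initializes both skill components with itself as owner and a key label, adding each to the Skills array.
; The Skill_0 and Skill_1 input actions print a debug line and call Fire on the matching component, which holds the skill logic.
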(event `EnhancedInput|/Game/_Project/CommonSystems/Input/Skill_0`
  (params (ActionValue :type Boolean) (ElapsedSeconds :type "Float (double-precision)") (TriggeredSeconds :type "Float (double-precision)") (InputAction :type "InputAction Object Reference" :default "/Game/_Project/CommonSystems/Input/Skill_0.Skill_0"))
  (:`Triggered`
    (`KismetSystemLibrary.PrintString` "It's a trap!")
    (`/Game/_Project/CommonSystems/Character_Skills/Character_Skill_BP.Fire` (`self.TrappSkillCooldown_BPC`))))

(event `self.ReceiveBeginPlay`
  (bind _trappskillcooldown_bpc (`self.TrappSkillCooldown_BPC`))
  (bind _expansiveforceskill_bpc (`self.ExpansiveForceSkill_BPC`))
  (`parent.ReceiveBeginPlay`)
  (`|ExecutionSequence`
    (:`then_0`
      (`self.InitializeHealth` (make `/Game/_Project/CommonSystems/HealthSystem/HealthData` 225.0 225.0)))
    (:`then_1`
      (`/Game/_Project/CommonSystems/Character_Skills/Character_Skill_BP.Initialize` _trappskillcooldown_bpc self "L SHIFT")
      (`KismetArrayLibrary.Array_Add` (`self.Skills`) _trappskillcooldown_bpc))
    (:`then_2`
      (`/Game/_Project/CommonSystems/Character_Skills/Character_Skill_BP.Initialize` _expansiveforceskill_bpc self "C")
      (`KismetArrayLibrary.Array_Add` (`self.Skills`) _expansiveforceskill_bpc))))

(event `EnhancedInput|/Game/_Project/CommonSystems/Input/Skill_1`
  (params (ActionValue :type Boolean) (ElapsedSeconds :type "Float (double-precision)") (TriggeredSeconds :type "Float (double-precision)") (InputAction :type "InputAction Object Reference" :default "/Game/_Project/CommonSystems/Input/Skill_1.Skill_1"))
  (:`Triggered`
    (`KismetSystemLibrary.PrintString` "It's NOT a trap!")
    (`/Game/_Project/CommonSystems/Character_Skills/Character_Skill_BP.Fire` (`self.ExpansiveForceSkill_BPC`))))

(event `self.ReceiveTick`
  (params (DeltaSeconds :type "Float (single-precision)"))
  (`parent.ReceiveTick` DeltaSeconds))

(fn `UserConstructionScript`
  (`parent.UserConstructionScript`))