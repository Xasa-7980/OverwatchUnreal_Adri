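; ExpansiveForce_BP is a Junkrat skill actor that knocks characters away from its position when it is destroyed.
; On Destroyed, it sphere-overlaps pawns within the RadialForce component's radius and launches each Character outward by Impulse, overriding its current velocity.
; Each launched character, with no exclusion for the owner, adds a fixed charge to the OwningCharacter's Ultimate if that owner is valid.
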(event `self.ReceiveDestroyed`
  (bind _outactors (`KismetSystemLibrary.SphereOverlapActors` (`self.K2_GetActorLocation`) (`RadialForceComponent.Radius` (`self.RadialForce`)) (`|MakeArray` "ObjectTypeQuery3" :!type "EObjectTypeQuery Enum") "/Script/Engine.Character"))
  (for _array_element _outactors
    (bind _ascharacter (cast `Character` _array_element))
    (`Character.LaunchCharacter` _ascharacter (* (`KismetMathLibrary.Normal` (- (`self.K2_GetActorLocation` _array_element) (`self.K2_GetActorLocation`))) (`self.Impulse`)) true true)
    (`/Engine/EditorBlueprintResources/StandardMacros.IsValid` (`self.OwningCharacter`)
      (:`Is Valid`
        (`/Game/_Project/CommonSystems/Character_Ultimate/Ultimate_BP.AddCharge` (`/Game/_Project/Characters/BaseCharacter_BP.Ultimate` (`self.OwningCharacter`)) 20.0)))))

(fn `UserConstructionScript`
  (`parent.UserConstructionScript`))