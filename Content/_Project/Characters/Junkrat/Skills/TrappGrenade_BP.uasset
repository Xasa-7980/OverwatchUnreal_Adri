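; Junkrat's trap skill actor, which roots the first character that overlaps it.
; On overlap with a BaseCharacter_BP, it latches a Trapped flag so only one victim is caught, then disables that character's movement.
; After the TrappedTime delay, it sets the victim's movement mode back to Walking, if the movement component is still valid, and destroys itself.
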(event `self.ReceiveActorBeginOverlap`
  (params (OtherActor :type "Actor Object Reference"))
  (if (not (`self.Trapped`))
    (bind _asbase_character_bp (cast `/Game/_Project/Characters/BaseCharacter_BP` OtherActor))
    (set `self.Trapped` true)
    (bind _charactermovement (`Character.CharacterMovement` _asbase_character_bp))
    (`CharacterMovementComponent.DisableMovement` _charactermovement)
    (`KismetSystemLibrary.Delay` (`self.TrappedTime`))
    (`/Engine/EditorBlueprintResources/StandardMacros.IsValid` _charactermovement
      (:`Is Valid`
        (`CharacterMovementComponent.SetMovementMode` _charactermovement "MOVE_Walking" 0))
      (:`Is Not Valid`
        _))
    (`self.K2_DestroyActor`)))

(event `self.ReceiveDestroyed`)

(fn `UserConstructionScript`
  (`parent.UserConstructionScript`))